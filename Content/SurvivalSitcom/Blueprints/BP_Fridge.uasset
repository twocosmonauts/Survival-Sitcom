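; BP_Fridge is an interactable fridge that starts eat requests and shows a current/max food count on a text render.
; Interact sends StartEatMessage, with itself and an amount, to every actor implementing BPI_Economic.
; BeginPlay sends an amount of zero and Interaction sends one.
; The EndEat event receives current and maximum food and writes them to the text.
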(event `self.ReceiveBeginPlay`
  (`self.interact` 0))

(event `self.Interaction`
  (`self.interact` 1))

(event `/Game/SurvivalSitcom/Blueprints/BPI_Economic.EndEat`
  (params (CurrentFood :type Integer) (MaxFood :type Integer))
  (`TextRenderComponent.K2_SetText` (`self.TextRender`) (`KismetTextLibrary.Conv_StringToText` (`KismetStringLibrary.Concat_StrStr` (`KismetStringLibrary.Conv_IntToString` CurrentFood) "/" (`KismetStringLibrary.Conv_IntToString` MaxFood)))))

(fn `interact`
  (params (HowMany :type Integer))
  (bind _outactors (`GameplayStatics.GetAllActorsWithInterface` "/Game/SurvivalSitcom/Blueprints/BPI_Economic.BPI_Economic_C"))
  (for _array_element _outactors
    (message `/Game/SurvivalSitcom/Blueprints/BPI_Economic.StartEat` _array_element self HowMany)))

(fn `UserConstructionScript`
  (`parent.UserConstructionScript`))