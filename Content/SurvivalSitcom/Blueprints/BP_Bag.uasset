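; BP_Bag is a bag actor that renders its contents through a scene capture and adds a WBP_Bag widget on BeginPlay.
; The SceneCaptureComponent2D is limited to showing only this actor and its child actors.
; Each tick, its Scene component copies the relative location of the first-person character's Scene component.
; Any child actor that begins overlapping the Box is destroyed with an "OUCH" debug print.
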(event `self.ReceiveBeginPlay`
  (`self.AddNewObjectInBag`)
  (bind _returnvalue (`|CreateWidget` "/Game/SurvivalSitcom/UI/WBP_Bag.WBP_Bag_C"))
  (`UserWidget.AddToViewport` _returnvalue 0)
  (bind _asbp_first_person_character (cast `/Game/StoryAdvTemplate/Blueprints/BP_FirstPersonCharacter` (`GameplayStatics.GetPlayerCharacter` 0)))
  (set `self.SceneBag` (`/Game/StoryAdvTemplate/Blueprints/BP_FirstPersonCharacter.Scene` _asbp_first_person_character)))

(event `self.ReceiveTick`
  (params (DeltaSeconds :type "Float (single-precision)"))
  (`SceneComponent.K2_SetRelativeTransform` (`self.Scene`) (`KismetMathLibrary.MakeTransform` (.location (`SceneComponent.GetRelativeTransform` (`self.SceneBag`))) (`KismetMathLibrary.MakeRotator` 0.0)) false false))

(event `self.Box.OnComponentBeginOverlap`
  (params (OverlappedComponent :type "PrimitiveComponent Object Reference") (OtherActor :type "Actor Object Reference") (OtherComp :type "PrimitiveComponent Object Reference") (OtherBodyIndex :type Integer) (bFromSweep :type Boolean) (SweepResult :type "HitResult Structure (by ref)"))
  (for _array_element (`self.GetAllChildActors` true)
    (if (== OtherActor _array_element)
      (`self.K2_DestroyActor` _array_element)
      (`KismetSystemLibrary.PrintString` "OUCH"))))

(fn `AddNewObjectInBag`
  (`SceneCaptureComponent.ShowOnlyActorComponents` (`self.SceneCaptureComponent2D`) self true))

(fn `UserConstructionScript`)