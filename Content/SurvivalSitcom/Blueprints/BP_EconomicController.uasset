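; BP_EconomicController tracks the day count, self-confidence and money in SurvivalSitcom.
; ChangeDay advances the current day and raises self-confidence by one, clamped between zero and the maximum set in EconomicParameters.
; GameDone adds a random payout to current money, ranging from zero up to the MoneyForGame limit in EconomicParameters.
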(event `ChangeDay`
  (`/Engine/EditorBlueprintResources/StandardMacros.IncrementInt` (`self.CurrentDay`)
    (:`  `
      (set `self.CurrentSelfConfidence` (`KismetMathLibrary.Clamp` (+ (`self.CurrentSelfConfidence`) 1) 0 (`.MaxSelfCOnfidence_8_85B17F7C4AF455A2A1422CA30889F5CA` (break `/Game/SurvivalSitcom/Blueprints/S_EconomicParameters` (`self.EconomicParameters`))))))))

(event `GameDone`
  (set `self.CurrentMoney` (+ (`self.CurrentMoney`) (`KismetMathLibrary.RandomFloatInRange` 0.0 (`.MoneyForGame_15_8AA1CB734B8577DEDF83AF9B6123254D` (break `/Game/SurvivalSitcom/Blueprints/S_EconomicParameters` (`self.EconomicParameters`)))))))

(fn `UserConstructionScript`)