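; BP_Goods is an item that can be added to the inventory and also appears as a physical object in the bag.
; Its construction script shuffles a mesh array and applies the first entry, randomizing each item's appearance.
; On AddItemtoInventory it runs parent logic, then spawns a child StaticMeshActor at BP_Bag's SpawnPoint with the same mesh.
; That copy simulates physics with overlaps and a slight downward impulse, and the bag is notified.
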(event `self.AddItemToInventory`
  (`parent.AddItemToInventory`)
  (bind _returnvalue (`GameplayStatics.GetActorOfClass` "/Game/SurvivalSitcom/Blueprints/BP_Bag.BP_Bag_C"))
  (bind _returnvalue_2 (`AddComponent|NODE_AddChildActorComponent-0` :`self` _returnvalue :`RelativeTransform` (`SceneComponent.GetRelativeTransform` (`/Game/SurvivalSitcom/Blueprints/BP_Bag.SpawnPoint` _returnvalue))))
  (`ChildActorComponent.SetChildActorClass` _returnvalue_2 "/Script/Engine.StaticMeshActor")
  (bind _asstatic_mesh_actor (cast `StaticMeshActor` (`ChildActorComponent.ChildActor` _returnvalue_2)))
  (`StaticMeshActor.SetMobility` _asstatic_mesh_actor "Movable")
  (bind _staticmeshcomponent (`StaticMeshActor.StaticMeshComponent` _asstatic_mesh_actor))
  (`StaticMeshComponent.SetStaticMesh` _staticmeshcomponent (`StaticMeshComponent.StaticMesh` (`self.Object`)))
  (`PrimitiveComponent.SetSimulatePhysics` _staticmeshcomponent true)
  (set `PrimitiveComponent.bGenerateOverlapEvents` true _staticmeshcomponent)
  (`PrimitiveComponent.AddImpulse` _staticmeshcomponent (0.0 0.0 -1.0) "None" false)
  (`/Game/SurvivalSitcom/Blueprints/BP_Bag.AddNewObjectInBag` _returnvalue))

(fn `UserConstructionScript`
  (bind _staticmesh (`self.StaticMesh`))
  (`parent.UserConstructionScript`)
  (`KismetArrayLibrary.Array_Shuffle` _staticmesh)
  (`StaticMeshComponent.SetStaticMesh` (`self.Object`) (`|GetArrayItem` _staticmesh)))