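; BP_WorkStation is an interactable workstation that advances game-completion progress, once per day.
; Interaction requires enough self-confidence, checked against both a hardcoded minimum and the threshold in BP_EconomicController's economic parameters.
; A random increment, its minimum derived from target completion days, updates a percentage text display; full progress calls GameDone and resets.
; ChangeDay resets the DoOnce gate, which is consumed before the parameter threshold check.
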(event `self.ReceiveBeginPlay`
  (bind _returnvalue (`GameplayStatics.GetActorOfClass` "/Game/SurvivalSitcom/Blueprints/BP_EconomicController.BP_EconomicController_C"))
  (bind _output_get (set `self.EconomController` _returnvalue))
  (set `self.Economic Parameters` (`/Game/SurvivalSitcom/Blueprints/BP_EconomicController.EconomicParameters` _output_get)))

(event `self.Interaction`
  (bind (_gamecomplitedays _moneyforgame _rent _maxselfconfidence _needselfconfidencetowork) (break `/Game/SurvivalSitcom/Blueprints/S_EconomicParameters` (`self.Economic Parameters`)))
  (if (not (< (`/Game/SurvivalSitcom/Blueprints/BP_EconomicController.CurrentSelfConfidence` (`self.EconomController`)) 3))
    (`/Engine/EditorBlueprintResources/StandardMacros.DoOnce` false :!label _label
      (:`Completed`
        (if (>= (`/Game/SurvivalSitcom/Blueprints/BP_EconomicController.CurrentSelfConfidence` (`self.EconomController`)) _needselfconfidencetowork)
          (set `self.CurrentWork` (`KismetMathLibrary.Clamp` (+ (`self.CurrentWork`) (`KismetMathLibrary.RandomIntegerInRange` (/ 100 _gamecomplitedays) 100)) 0 100))
          (`TextRenderComponent.K2_SetText` (`self.TextRender`) (`KismetTextLibrary.Conv_StringToText` (`KismetStringLibrary.Concat_StrStr` (`KismetStringLibrary.Conv_IntToString` (`self.CurrentWork`)) "/100%")))
          (if (>= (`self.CurrentWork`) 100)
            (`/Game/SurvivalSitcom/Blueprints/BP_EconomicController.GameDone` (`self.EconomController`))
            (set `self.CurrentWork` 0)))))))

(event `/Game/SurvivalSitcom/Blueprints/BPI_Economic.ChangeDay`
  (goto _label :!via `Reset`))

(fn `UserConstructionScript`
  (`parent.UserConstructionScript`))